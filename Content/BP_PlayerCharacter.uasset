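; Player character Blueprint that sets up the main HUD and camera limits when play begins.
; BeginPlay adds the WBP_MainHUD widget to the viewport and narrows the camera manager's view pitch range.
; A debug Tab key flip-flops global time dilation between slow motion and normal speed.
; The construction script hides the mesh's left and right weapon bones and its grenade bone.
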(event EventBeginPlay
  (bind _returnvalue (Game|GetPlayerCameraManager 0))
  (bind _returnvalue_2 (UserInterface|CreateWidget "/Game/Core/UI/WBP_MainHUD.WBP_MainHUD_C"))
  (UserInterface|Viewport|AddtoViewport _returnvalue_2 0)
  ;[0.15 0.15 0.15 0.5] a little camera tweak
  (Variables|/Script/Engine.PlayerCameraManager|SetViewPitchMax _returnvalue 4e+01)
  (Variables|/Script/Engine.PlayerCameraManager|SetViewPitchMin _returnvalue -6e+01))

(event Input|KeyboardEvents|DebugKeyTab
  (params (Key :type Key%20Structure :default "None") (ActionValue :type Input%20Action%20Value%20Structure))
  (:Pressed
    (Utilities|FlowControl|FlipFlop
      (:A
        (Utilities|Time|SetGlobalTimeDilation 0.2))
      (:B
        (Utilities|Time|SetGlobalTimeDilation 1.0)))))

(fn ConstructionScript
  (Components|SkinnedMesh|HideBonebyName (Variables|Character|GetMesh) "weapon_r" "PBO_None")
  (Components|SkinnedMesh|HideBonebyName (Variables|Character|GetMesh) "weapon_l" "PBO_None")
  (Components|SkinnedMesh|HideBonebyName (Variables|Character|GetMesh) "grenade" "PBO_None"))