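; Actor component that gives a Character physics-driven hit reactions using a physical animation component it creates at BeginPlay.
; HitReaction extends a timer, simulates bodies below the pelvis with the "HitReaction" profile and applies an impulse along the trace direction.
; Tick decays the timer, using it as physics blend weight, then stops simulation and ticking and sets query-only collision.
; TogglePhysicalAnimation enables physics collision and simulation without an impulse.
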(event `self.ReceiveTick`
  (params (DeltaSeconds :type "Float (single-precision)"))
  (set `self.HitReactionTimeRemaining` (- (`KismetMathLibrary.FInterpTo` (`self.HitReactionTimeRemaining`) 0.0 0.0 1.0) (* DeltaSeconds 0.1)))
  (if (<= (`self.HitReactionTimeRemaining`) 0.0)
    (set `self.HitReactionTimeRemaining` 0.0)
    (`SkeletalMeshComponent.SetAllBodiesBelowSimulatePhysics` (`self.Mesh`) "pelvis" false true)
    (`self.SetComponentTickEnabled` false)
    (`PrimitiveComponent.SetCollisionEnabled` (`self.Mesh`) "QueryOnly")
    (else
      ; ?
      (`SkeletalMeshComponent.SetAllBodiesBelowPhysicsBlendWeight` (`self.Mesh`) "pelvis" (`KismetMathLibrary.FMin` (`self.HitReactionTimeRemaining`) 1.0) false true))))

(event `self.ReceiveBeginPlay`
  (bind _returnvalue (`|AddComponentByClass` (`self.GetOwner`) "/Script/Engine.PhysicalAnimationComponent"))
  (bind _output_get (set `self.PhysicalAnimationComponent` _returnvalue))
  (bind _ascharacter (cast `Character` (`self.GetOwner`)))
  (bind _mesh (`Character.Mesh` _ascharacter))
  (`PhysicalAnimationComponent.SetSkeletalMeshComponent` _output_get _mesh)
  (set `self.Mesh` _mesh))

(event `HitReaction`
  (params (Hit :type "HitResult Structure"))
  (bind (_bblockinghit _binitialoverlap _time _distance _location _impactpoint _normal _impactnormal _physmat _hitactor _hitcomponent _hitbonename _bonename _hititem _elementindex _faceindex _tracestart _traceend) (`GameplayStatics.BreakHitResult` Hit))
  (`self.SetComponentTickEnabled` true)
  (set `self.HitReactionTimeRemaining` (+ 2.0 (`self.HitReactionTimeRemaining`)))
  (`PhysicalAnimationComponent.ApplyPhysicalAnimationProfileBelow` (`self.PhysicalAnimationComponent`) "pelvis" "HitReaction" false false)
  (`SkeletalMeshComponent.SetAllBodiesBelowSimulatePhysics` (`self.Mesh`) "pelvis" true false)
  (`PrimitiveComponent.AddImpulse` (`self.Mesh`) (* (`KismetMathLibrary.Normal` (- _traceend _tracestart)) 5000.0) (select `bool` (== _hitbonename "pelvis") :`false` _hitbonename) true))

(event `TogglePhysicalAnimation`
  (`PrimitiveComponent.SetCollisionEnabled` (`self.Mesh`) "QueryAndPhysics")
  (`PhysicalAnimationComponent.ApplyPhysicalAnimationProfileBelow` (`self.PhysicalAnimationComponent`) "pelvis" "HitReaction" false false)
  (`SkeletalMeshComponent.SetAllBodiesBelowSimulatePhysics` (`self.Mesh`) "pelvis" true false))